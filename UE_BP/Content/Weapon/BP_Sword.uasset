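; BP_Sword is a melee sword weapon that moves between holster and hand sockets on equip and plays combo attacks.
; DoAction starts the first action when the owner is idle via IState, or queues the next hit if the combo window is open; BeginAction then advances the montage index.
; EndAction resets the combo, idle state and weapon movement.
; Capsule collision starts disabled, and its overlap handler filters owner and self without applying any effect.
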(event OnComponentBeginOverlap(Capsule)
  (params (OverlappedComponent :type Primitive%20Component%20Object%20Reference) (OtherActor :type Actor%20Object%20Reference) (OtherComp :type Primitive%20Component%20Object%20Reference) (OtherBodyIndex :type Integer) (bFromSweep :type Boolean) (SweepResult :type Hit%20Result%20Structure%20%28by%20ref%29))
  ;[1 1 1] BeginOverlap
  (if (and (!= OtherActor (Variables|Default|GetOwnerCharacter)) (!= OtherActor self))
    _))

(event Custom|Lock_EnableCombo
  ;[1 1 1] Combo
  (Variables|Default|SetEnable false))

(event Custom|UnLock_EnableCombo
  ;[1 1 1] Combo
  (Variables|Default|SetEnable true))

(event EventDoAction
  (bind _ownercharacter (Variables|Default|GetOwnerCharacter))
  ;[1 1 1] DoAction
  (|CallParentFunction)
  (if (CallFunction|IsExistAction)
    (if (Variables|Default|GetEnable)
      (Variables|Default|SetEnable false)
      (Variables|Default|SetExist true)
      (elif (Utilities|DoesObjectImplementInterface _ownercharacter "/Game/Interfaces/IState.IState_C")
        (bind _result (Class|IState|IsStateIdle(Message) _ownercharacter))
        (if _result
          (Class|IState|SetStateAction(Message) _ownercharacter)
          (CallFunction|PlayAction))))))

(event EventBeginAction
  ;[1 1 1] BeginAction
  (|CallParentFunction)
  (if (Variables|Default|GetExist)
    (Variables|Default|SetExist false)
    (Animation|StopAnimMontage (Variables|Default|GetOwnerCharacter) 0)
    (Math|Integer|IncrementInt (Variables|Default|GetIndex)
      (:%20%20
        (CallFunction|PlayAction (Variables|Default|GetIndex))))))

(event EventEndAction
  (bind _ownercharacter (Variables|Default|GetOwnerCharacter))
  (bind _ownercharacter_2 (Variables|Default|GetOwnerCharacter))
  ;[1 1 1] EndAction
  (|CallParentFunction)
  (Variables|Default|SetIndex 0)
  (Animation|StopAnimMontage _ownercharacter_2 0)
  (if (Utilities|DoesObjectImplementInterface _ownercharacter_2 "/Game/Interfaces/IState.IState_C")
    (Class|IState|SetStateIdle(Message) _ownercharacter)
    (if (Utilities|DoesObjectImplementInterface _ownercharacter "/Game/Interfaces/IWeapon.IWeapon_C")
      (Class|IWeapon|SetWeaponMove(Message) (Variables|Default|GetOwnerCharacter)))))

(event EventBeginPlay
  ;[1 1 1] BeginPlay
  (|CallParentFunction)
  (CallFunction|AttachtoOwnerCharacter "Holster_Sword")
  (CallFunction|OffCollsion))

(event EventBeginEquip
  ;[1 1 1] Equip
  (|CallParentFunction)
  (CallFunction|AttachtoOwnerCharacter "Hand_Sword"))

(event EventEndEquip
  ;[1 1 1] Equip
  (|CallParentFunction)
  (CallFunction|AttachtoOwnerCharacter "Holster_Sword"))

(fn ConstructionScript
  (|CallParentFunction))

(fn OnCollision
  (Collision|SetCollisionEnabled (Variables|Default|GetCapsule) "QueryAndPhysics"))

(fn OffCollsion
  (Collision|SetCollisionEnabled (Variables|Default|GetCapsule) "NoCollision"))