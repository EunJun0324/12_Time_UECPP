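; BP_SubAction_Launcher is a weapon sub-action that plays the launcher montage on its owning character.
; DoSubAction talks to the owner through the IState interface, proceeding only when the state is idle and the switching check returns true.
; It then sets the Action state and plays the montage and rate from ActionData.
; EndSubAction returns the owner to Idle, while BeginPlay and BeginSubAction only call the parent.
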(event EventBeginPlay
  (params (InOwner :type Character%20Object%20Reference))
  (|CallParentFunction InOwner))

(event EventBeginSubAction
  (|CallParentFunction))

(event EventDoSubAction
  (bind _actiondata (Variables|Default|GetActionData))
  (bind _ownercharacter (Variables|Default|GetOwnerCharacter))
  (|CallParentFunction)
  (if (Utilities|DoesObjectImplementInterface _ownercharacter "/Game/Interfaces/IState.IState_C")
    (bind _result (Class|IState|IsStateIdle(Message) _ownercharacter))
    (if _result
      (bind _result_2 (Class|IWeapon|IsSwitching(Message) _ownercharacter))
      (if _result_2
        (Class|IState|SetStateAction(Message) _ownercharacter)
        (Animation|PlayAnimMontage (Variables|Default|GetOwnerCharacter) (.montage _actiondata) (.playratio _actiondata) "None")))))

(event EventEndSubAction
  (bind _ownercharacter (Variables|Default|GetOwnerCharacter))
  (|CallParentFunction)
  (if (Utilities|DoesObjectImplementInterface _ownercharacter "/Game/Interfaces/IState.IState_C")
    (Class|IState|SetStateIdle(Message) _ownercharacter)))